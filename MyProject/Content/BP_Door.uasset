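; Door actor that swings its static mesh when a BP_FirstPersonCharacter enters its box trigger.
; Begin overlap replays Timeline_1 from the start, setting the mesh's world yaw from its track.
; End overlap does nothing, and the E key handler only clears EndedAnimation before an empty branch.
; Older open and close timelines with IsOpened and IsOverlapping state remain in the graph but never run.
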(event `self.ReceiveBeginPlay`)

(event `self.Box.OnComponentEndOverlap`
  (params (OverlappedComponent :type "PrimitiveComponent Object Reference") (OtherActor :type "Actor Object Reference") (OtherComp :type "PrimitiveComponent Object Reference") (OtherBodyIndex :type Integer)))

(event `Key|E`
  (params (Key :type "Key Structure"))
  (:`Pressed`
    (if (and (`self.isOverlapping`) (`self.endedAnimation`))
      (set `self.endedAnimation` false)
      (if (`self.isOpened`)
        _))))

(event `self.Box.OnComponentBeginOverlap`
  (params (OverlappedComponent :type "PrimitiveComponent Object Reference") (OtherActor :type "Actor Object Reference") (OtherComp :type "PrimitiveComponent Object Reference") (OtherBodyIndex :type Integer) (bFromSweep :type Boolean) (SweepResult :type "HitResult Structure (by ref)"))
  (cast `/Game/FirstPerson/Blueprints/BP_FirstPersonCharacter` OtherActor)
  (bind (_direction _newtrack_0) (`Timeline|Timeline_1` :!via `PlayFromStart`)
    (:`Update`
      (`SceneComponent.K2_SetWorldRotation` (`self.StaticMesh`) (`KismetMathLibrary.MakeRotator` 0.0 0.0 _newtrack_0) false false))))

(fn `UserConstructionScript`)