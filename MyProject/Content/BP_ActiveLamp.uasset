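; BP_ActiveLamp is a proximity lamp that lights up while the first-person player character is inside its trigger box.
; On overlap begin, after a short delay, it swaps the cylinder to a yellow light material and turns on the spotlight.
; On overlap end, it restores the gray grid material and zeroes the spotlight intensity immediately.
; The construction script starts the spotlight switched off.
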(event `self.Box.OnComponentBeginOverlap`
  (params (OverlappedComponent :type "PrimitiveComponent Object Reference") (OtherActor :type "Actor Object Reference") (OtherComp :type "PrimitiveComponent Object Reference") (OtherBodyIndex :type Integer) (bFromSweep :type Boolean) (SweepResult :type "HitResult Structure (by ref)"))
  (cast `/Game/FirstPerson/Blueprints/BP_FirstPersonCharacter` OtherActor)
  (`KismetSystemLibrary.Delay` 0.2)
  (`PrimitiveComponent.SetMaterial` (`self.Cylinder`) 0 "/Game/MatsAndTextures/M_YellowLight.M_YellowLight")
  (`LightComponent.SetIntensity` (`self.SpotLight`) 5000.0))

(event `self.Box.OnComponentEndOverlap`
  (params (OverlappedComponent :type "PrimitiveComponent Object Reference") (OtherActor :type "Actor Object Reference") (OtherComp :type "PrimitiveComponent Object Reference") (OtherBodyIndex :type Integer))
  (cast `/Game/FirstPerson/Blueprints/BP_FirstPersonCharacter` OtherActor)
  (`PrimitiveComponent.SetMaterial` (`self.Cylinder`) 0 "/Game/LevelPrototyping/Materials/MI_PrototypeGrid_Gray.MI_PrototypeGrid_Gray")
  (`LightComponent.SetIntensity` (`self.SpotLight`) 0.0))

(fn `UserConstructionScript`
  (`LightComponent.SetIntensity` (`self.SpotLight`) 0.0))